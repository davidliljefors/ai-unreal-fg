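; Exploding NPC that turns its melee attack into a suicide blast.
; MeleeAttack zeroes its base speed and runs a timeline that shifts the body color through a dynamic material instance as a fuse.
; If still alive when the timeline finishes, a single sphere trace sends melee damage via ShotMessage to the first actor hit.
; The NPC then ragdolls, hit or miss, and plays an explosion sound.
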(event EventBeginPlay
  (|CallParentFunction) ; This node is disabled and will not be called.\nDrag off pins to build functionality.
)

(event EventMeleeAttack
  (bind _returnvalue (Transformation|GetActorLocation))
  (bind _mesh (Variables|Character|GetMesh))
  (Variables|Default|SetBaseSpeed 0.0)
  (bind _returnvalue_2 (Rendering|Material|CreateDynamicMaterialInstance _mesh 0 (Rendering|Material|GetMaterial _mesh 0) "None" :!class /Script/Engine.PrimitiveComponent))
  (bind _returnvalue_3 (Rendering|Material|GetVectorParameterValue _returnvalue_2 "BodyColor" :!class /Script/Engine.MaterialInstanceDynamic))
  (bind _float_track (Timeline|Timeline_0 Play)
    (:Update
      (Rendering|Material|SetVectorParameterValue _returnvalue_2 "BodyColor" (Utilities|Struct|MakeLinearColor _float_track (* _float_track 0.5) (.b _returnvalue_3) 1.0) :!class /Script/Engine.MaterialInstanceDynamic))
    (:Finished
      (if (Variables|Default|GetbIsAlive)
        (bind (_outhit _returnvalue_4) (Collision|SphereTraceByChannel _returnvalue (+ _returnvalue 1.0) 3e+02 "TraceTypeQuery3" false 0 "None"))
        (if _returnvalue_4
          (Class|BPIInteractable|Shot(Message) (.hitactor _outhit) (Variables|Default|GetMeleeDamage) self (.impactpoint _outhit) "None")
          (CallFunction|DieasRagdoll "0, 0, 0" "None")
          (else
            (CallFunction|DieasRagdoll "0, 0, 0" "None")))
        (Audio|PlaySoundatLocation "/Game/StarterContent/Audio/Explosion02.Explosion02" (Transformation|GetActorLocation) "0, 0, 0" 3.0 1.0 0.0 "/Game/MilitaryWeapSilver/Sound/SniperRifle/Wavs/AttenuationTest.AttenuationTest" 0 0)))))

(fn ConstructionScript
  (|CallParentFunction))