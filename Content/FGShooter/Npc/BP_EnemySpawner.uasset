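; BP_EnemySpawner spawns enemy NPCs at its arrow, avoiding spawns in the player's view.
; TrySpawn traces on the Camera channel to the player, failing only if it hits BP_SourcePlayer with hit normal and actor forward roughly aligned (player facing the spawner).
; Otherwise SpawnAI creates the override or default Enemy class, assigns its PatrolPath and activates its AIC_Npc controller.
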(fn ConstructionScript)

(fn TrySpawn
  (params (Override%20Spawn%20Class :type BP%20Npc%20Class%20Reference))
  (bind _outhit (Collision|LineTraceByChannel (Transformation|GetWorldLocation (Variables|Default|GetArrow)) (Transformation|GetWorldLocation (Variables|/Script/Engine.Actor|GetRootComponent (Game|GetPlayerCharacter 0))) "TraceTypeQuery2" false 0 "None"))
  (Utilities|IsValid (.hitactor _outhit)
    (:Is%20Valid
      (if (Math|Float|InRange(Float) (Math|Vector|DotProduct (.normal _outhit) (Math|Rotator|GetRotationXVector (Transformation|GetActorRotation (.hitactor _outhit)))) -1.0 0.5)
        _
        (elif (not (== (Utilities|GetClass (.hitactor _outhit)) "/Game/FGShooter/BP_SourcePlayer.BP_SourcePlayer_C"))
          _
          (else
            (return false 0))))
      (if (Utilities|IsValidClass Override%20Spawn%20Class)
        (bind _returnvalue (Utilities|SpawnAI Override%20Spawn%20Class))
        (return true _returnvalue)
        (else
          (bind _returnvalue_2 (Utilities|SpawnAI (Variables|SpawnParameters|GetEnemy)))
          (return true _returnvalue_2))))
    (:Is%20Not%20Valid
      (if (Utilities|IsValidClass Override%20Spawn%20Class)
        (bind _returnvalue_3 (Utilities|SpawnAI Override%20Spawn%20Class))
        (return true _returnvalue_3)
        (else
          (bind _returnvalue_4 (Utilities|SpawnAI (Variables|SpawnParameters|GetEnemy)))
          (return true _returnvalue_4))))))