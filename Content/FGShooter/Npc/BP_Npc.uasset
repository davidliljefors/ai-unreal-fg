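; Zombie NPC for the shooter, with randomized health, speed and melee damage, plus a looping idle moan while alive.
; MeleeAttack plays a montage, then after a short delay sphere-traces forward and sends ShotMessage to the hit actor.
; Shot applies damage with a headshot multiplier and adds GameState score capped at remaining health.
; Death ragdolls the mesh with an impulse, clears the blackboard alive flag, signals the kill and sometimes drops an item.
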(event EventMeleeAttack
  (bind _returnvalue (Transformation|GetActorLocation))
  ;[1 1 1] do melee attack
  (Animation|Montage|PlayMontage (Variables|Character|GetMesh) "/Game/FGShooter/Npc/AM_BasicAttack.AM_BasicAttack" 2.0
    (:then
      (Utilities|FlowControl|Delay 0.25)
      (if (Variables|Default|GetbIsAlive)
        (bind _outhit (Collision|SphereTraceByChannel _returnvalue (+ _returnvalue (* (Transformation|GetActorForwardVector) (Variables|Default|GetMeleeRange))) 75.0 "TraceTypeQuery3" false 0 "None" true "(R=1.000000,G=0.000000,B=0.000000,A=1.000000)" "(R=0.000000,G=1.000000,B=0.000000,A=1.000000)" 1.0))
        (Class|BPIInteractable|Shot(Message) (.hitactor _outhit) (Variables|Default|GetMeleeDamage) self (.impactpoint _outhit) (.hitbonename _outhit))))))

(event EventBeginPlay
  ;[1 1 1] Add some variety to gameplay and randomize combat values
  (Variables|Default|SetHealth (* (Variables|Default|GetHealth) (Math|Random|RandomFloatinRange 0.9 1.1)))
  (Variables|Default|SetBaseSpeed (* (Variables|Default|GetBaseSpeed) (Math|Random|RandomFloatinRange 0.9 1.1)))
  (Variables|Default|SetMeleeDamage (* (Variables|Default|GetMeleeDamage) (Math|Random|RandomFloatinRange 0.9 1.1)))
  ;[1 1 1] Loop to make some zombe sound effects
  (Utilities|FlowControl|Delay (Math|Random|RandomFloatinRange 4.0 14.0) :!label _label)
  (if (Variables|Default|GetbIsAlive)
    (CallFunction|ZombieNoise)
    (goto _label)))

(event EventShot
  (params (Damage :type Float%20%28single-precision%29) (Instigator :type Actor%20Object%20Reference) (Hit%20Point :type Vector :default "0, 0, 0") (Bone%20Hit :type Name :default "None"))
  (bind _returnvalue (Utilities|Name|Equal(Name) Bone%20Hit "head"))
  ;[0.2708 0.2708 0.2708] Get shot, if health < 0, enable ragdoll physics and become dead
  (if (Variables|Default|GetbIsAlive)
    (Utilities|AddScore Damage _returnvalue)
    (if _returnvalue
      (Variables|Default|SetHealth (- (Variables|Default|GetHealth) (* Damage (Variables|Default|GetHeadshot%20Dmg%20Mult))))
      (else
        (Variables|Default|SetHealth (- (Variables|Default|GetHealth) Damage))))
    (Effects|SpawnEmitteratLocation "/Game/MilitaryWeapSilver/FX/P_Impact_Stone_Large_01.P_Impact_Stone_Large_01" Hit%20Point)
    (if (<= (Variables|Default|GetHealth) 0.0)
      (CallFunction|DieasRagdoll Hit%20Point Bone%20Hit))))

(fn ConstructionScript)

(fn ZombieNoise
  (bind _idlesounds (Variables|Default|GetIdleSounds))
  (Audio|PlaySoundatLocation (Utilities|Array|Get(acopy) _idlesounds (Math|Random|RandomIntegerinRange 0 (- (Utilities|Array|Length _idlesounds) 1))) (Transformation|GetWorldLocation (Variables|Default|GetCenter)) "0, 0, 0" 0.6 1.0 0.0 "/Game/FGShooter/Npc/Sounds/ATT_Zombie.ATT_Zombie" 0 0)
  (return))

(fn DieasRagdoll
  (params (Hit%20Location :type Vector) (Bone%20Hit :type Name))
  (bind _mesh (Variables|Character|GetMesh))
  (bind _returnvalue (Transformation|GetWorldTransform _mesh))
  (Effects|SpawnEmitteratLocation "/Game/StarterContent/Particles/P_Explosion.P_Explosion" (Transformation|GetWorldLocation (Variables|Default|GetCenter)))
  (Audio|PlaySoundatLocation "/Game/StarterContent/Audio/Explosion01.Explosion01" (Transformation|GetActorLocation) "0, 0, 0" 0.45 1.0 0.0 "/Game/MilitaryWeapSilver/Sound/SniperRifle/Wavs/AttenuationTest.AttenuationTest" 0 0)
  (Class|SkeletalMeshComponent|SetAllBodiesBelowSimulatePhysics (Variables|Character|GetMesh) (Utilities|Name|MakeLiteralName "pelvis") true true)
  (Class|PrimitiveComponent|AddForceatLocation (Variables|Character|GetMesh) (Math|Vector|RotateVector (Math|Vector|MakeVector -1e+06 0.0 2e+06) (Transformation|GetWorldRotation (Variables|Collision|GetCapsuleComponent))) Hit%20Location Bone%20Hit)
  (AI|Components|Blackboard|SetValueasBool (AI|GetBlackboard 0) (Utilities|Name|MakeLiteralName "bIsAlive") false)
  (Collision|SetCollisionEnabled (Variables|Collision|GetCapsuleComponent) "NoCollision")
  (Variables|Default|SetbIsAlive false)
  (Default|CallOnKilled)
  (Actor|SetLifeSpan 7.0)
  (if (> (Math|Random|RandomFloat) 0.7)
    (Game|SpawnActorfromClass (Variables|Default|GetDropItem) (Math|Transform|MakeTransform (.location _returnvalue) (.rotation _returnvalue) "1,1,1") "AdjustIfPossibleButAlwaysSpawn" 0 0)))