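; Enemy NPC Blueprint with a melee attack and health-based death.
; MeleeAttack plays a montage, waits briefly to time the strike, then runs a short forward sphere trace with debug drawing and sends ShotMessage damage to the hit actor.
; The Shot event subtracts incoming damage from Health and, at zero or below, spawns an explosion effect and sound before destroying the actor.
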(event EventMeleeAttack
  (bind _returnvalue (Transformation|GetActorLocation))
  ;[1 1 1] do melee attack
  (Animation|Montage|PlayMontage (Variables|Character|GetMesh) "/Game/FGShooter/Npc/AM_BasicAttack.AM_BasicAttack"
    (:then
      (Utilities|FlowControl|Delay 0.6)
      (bind _outhit (Collision|SphereTraceByChannel _returnvalue (+ _returnvalue (* (Transformation|GetActorForwardVector) 5e+01)) 5e+01 "TraceTypeQuery2" false 0 "ForDuration" true "(R=1.000000,G=0.000000,B=0.000000,A=1.000000)" "(R=0.000000,G=1.000000,B=0.000000,A=1.000000)" 1.0))
      (Class|BPIInteractable|Shot(Message) (.hitactor _outhit) 15.0 self "0, 0, 0" "None"))))

(event EventShot
  (params (Damage :type Float%20%28single-precision%29) (Instigator :type Actor%20Object%20Reference) (Hit%20Point :type Vector :default "0, 0, 0") (Bone%20Hit :type Name :default "None"))
  ;[1 1 1] get shot event
  (bind _output_get (Variables|Default|SetHealth (- (Variables|Default|GetHealth) Damage)))
  (if (<= _output_get 0.0)
    (Effects|SpawnEmitteratLocation "/Game/StarterContent/Particles/P_Explosion.P_Explosion" (Transformation|GetActorLocation))
    (Audio|PlaySoundatLocation "/Game/StarterContent/Audio/Explosion01.Explosion01" (Transformation|GetActorLocation) "0, 0, 0" 1.0 1.0 0.0 0 0 0)
    (Actor|DestroyActor)))

(fn ConstructionScript)