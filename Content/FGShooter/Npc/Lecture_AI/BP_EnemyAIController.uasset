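; BP_EnemyAIController is the AI controller for enemy NPCs, running the BT_Enemy behavior tree on possession.
; Its perception update event is empty, so sensing currently has no effect on the Blackboard.
; Disconnected logic would set TargetPlayer to the player character when successfully sensed and clear it otherwise, but it never runs.
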(event OnTargetPerceptionUpdated(AIPerception)
  (params (Actor :type Actor%20Object%20Reference) (Stimulus :type AI%20Stimulus%20Structure)))

(event EventPossess
  (params (PossessedPawn :type Pawn%20Object%20Reference))
  (AI|RunBehaviorTree "/Game/FGShooter/Npc/Lecture_AI/BT_Enemy.BT_Enemy"))

(fn ConstructionScript)