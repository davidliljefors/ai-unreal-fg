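; Spawn manager that runs multi-wave NPC encounters through a set of spawners, handing them a shared patrol path on BeginPlay.
; Each wave spawns weighted-random NPC types one by one at random spawners, retrying failed spawns after a short delay.
; Kill callbacks track living enemies and advance waves on clear, signalling completion after the last.
; A retriggerable timeout forces stalled waves onward, using SkipCount to swallow later clear signals.
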(event Custom|SpawnGroup
  (params (Amount :type Integer) (SpawnData :type Array%20of%20F%20Enemy%20Spawn%20Data%20Structures))
  (bind _spawners (Variables|Spawning|GetSpawners))
  ;[1 1 1] Handle spawning of a group / wave
  (if (not (Variables|Default|GetbSpawningGroup))
    (Variables|Default|SetEnemiesLeftToSpawn Amount)
    (Variables|Default|SetbSpawningGroup true)
    (bind (_success _spawned_ai) (Default|TrySpawn (Utilities|Array|Get(acopy) _spawners (Math|Random|RandomIntegerinRange 0 (- (Utilities|Array|Length _spawners) 1))) (CallFunction|GetWeightedNpc SpawnData)))
    (if _success
      (Math|Integer|IncrementInt (Variables|Default|GetEnemiesAlive)
        (:%20%20
          (bind _asbp_npc (Utilities|Casting|CastToBP_Npc _spawned_ai))
          (EventDispatchers|BindEventtoOnKilled _asbp_npc (delegate Custom|EnemyKilled))
          (Utilities|FlowControl|Delay (Variables|Default|GetSpawnDelay))
          (bind _result (Math|Integer|DecrementInt (Variables|Default|GetEnemiesLeftToSpawn))
            (:%20%20
              (if (> _result 0)
                (CallFunction|Respawn)
                (else
                  (Variables|Default|SetbSpawningGroup false)
                  (if (== (Variables|Default|GetEnemiesAlive) 0)
                    (if (> (Variables|Default|GetSkipCount) 0)
                      (Math|Integer|DecrementInt (Variables|Default|GetSkipCount))
                      (else
                        (Default|CallSpawnerDone))))))))))
      (else
        (Utilities|FlowControl|Delay 0.1)
        (CallFunction|Respawn)))))

(event Custom|EnemyKilled
  (Math|Integer|DecrementInt (Variables|Default|GetEnemiesAlive)
    (:%20%20
      (if (== (Variables|Default|GetEnemiesAlive) 0)
        (if (not (Variables|Default|GetbSpawningGroup))
          (if (> (Variables|Default|GetSkipCount) 0)
            (Math|Integer|DecrementInt (Variables|Default|GetSkipCount))
            (else
              (Default|CallSpawnerDone))))))))

(event Custom|respawn
  (bind _spawners (Variables|Spawning|GetSpawners))
  ;[1 1 1] Handle spawning of a group / wave
  (bind (_success _spawned_ai) (Default|TrySpawn (Utilities|Array|Get(acopy) _spawners (Math|Random|RandomIntegerinRange 0 (- (Utilities|Array|Length _spawners) 1))) (CallFunction|GetWeightedNpc (stale Custom|SpawnGroup SpawnData))))
  (if _success
    (Math|Integer|IncrementInt (Variables|Default|GetEnemiesAlive)
      (:%20%20
        (bind _asbp_npc (Utilities|Casting|CastToBP_Npc _spawned_ai))
        (EventDispatchers|BindEventtoOnKilled _asbp_npc (delegate Custom|EnemyKilled))
        (Utilities|FlowControl|Delay (Variables|Default|GetSpawnDelay))
        (bind _result (Math|Integer|DecrementInt (Variables|Default|GetEnemiesLeftToSpawn))
          (:%20%20
            (if (> _result 0)
              (CallFunction|Respawn)
              (else
                (Variables|Default|SetbSpawningGroup false)
                (if (== (Variables|Default|GetEnemiesAlive) 0)
                  (if (> (Variables|Default|GetSkipCount) 0)
                    (Math|Integer|DecrementInt (Variables|Default|GetSkipCount))
                    (else
                      (Default|CallSpawnerDone))))))))))
    (else
      (Utilities|FlowControl|Delay 0.1)
      (CallFunction|Respawn))))

(event Custom|Spawn%20Waves
  (params (Spawn%20Data :type F%20Spawn%20Wave%20Structure))
  ;[1 1 1] Handle spawning of multiple waves
  (if (not (Variables|Default|GetbSpawning))
    (Variables|Default|SetbSpawning true)
    (EventDispatchers|BindEventtoSpawnerDone (delegate Custom|NextWave))
    (CallFunction|SpawnGroup (Utilities|Array|Get(acopy) (.spawnsforeachwave Spawn%20Data) (Variables|Default|GetCurrentWave)) (.spawndata Spawn%20Data))
    (Variables|Default|SetCahcedWave (Variables|Default|GetCurrentWave))
    (Utilities|FlowControl|RetriggerableDelay (.maxtimebetweenwaves Spawn%20Data))
    (if (== (Variables|Default|GetCahcedWave) (Variables|Default|GetCurrentWave))
      (CallFunction|NextWave)
      (Math|Integer|IncrementInt (Variables|Default|GetSkipCount)))))

(event Custom|NextWave
  ;[1 1 1] Handle spawning of multiple waves
  (Development|PrintString (Utilities|String|Append "Wave " (Utilities|String|ToString(Integer) (+ (Variables|Default|GetCurrentWave) 1)) " cleared!"))
  (Math|Integer|IncrementInt (Variables|Default|GetCurrentWave)
    (:%20%20
      (if (>= (Variables|Default|GetCurrentWave) (.wavecount (stale Custom|Spawn%20Waves Spawn%20Data)))
        (EventDispatchers|UnbindEventfromSpawnerDone (delegate Custom|NextWave))
        (Default|CallSpawnWaveDone)
        (Variables|Default|SetbSpawning false)
        (Variables|Default|SetCurrentWave 0)
        (else
          (CallFunction|SpawnGroup (Utilities|Array|Get(acopy) (.spawnsforeachwave (stale Custom|Spawn%20Waves Spawn%20Data)) (Variables|Default|GetCurrentWave)) (.spawndata (stale Custom|Spawn%20Waves Spawn%20Data)))
          (Variables|Default|SetCahcedWave (Variables|Default|GetCurrentWave))
          (Utilities|FlowControl|RetriggerableDelay (.maxtimebetweenwaves (stale Custom|Spawn%20Waves Spawn%20Data)))
          (if (== (Variables|Default|GetCahcedWave) (Variables|Default|GetCurrentWave))
            (CallFunction|NextWave)
            (Math|Integer|IncrementInt (Variables|Default|GetSkipCount))))))))

(event EventBeginPlay
  (bind _patrol_path (Variables|Default|GetPatrol%20Path)
    (:then
      (for _array_element (Variables|Spawning|GetSpawners)
        (Variables|/Game/FGShooter/Npc/BP_EnemySpawner.BP_EnemySpawner_C|SetPatrolPath _array_element _patrol_path)))
    (:else)))

(fn ConstructionScript)

(fn GetWeightedNpc
  (params (Spawn%20Data :type Array%20of%20F%20Enemy%20Spawn%20Data%20Structures))
  (for _array_element Spawn%20Data
    (LocalVariables|SetTotalWeight (+ (LocalVariables|GetTotalWeight) (.Spawnweight (Utilities|Struct|BreakFEnemySpawnData _array_element)))))
  (LocalVariables|SetRandomValue (Math|Random|RandomFloatinRange 0.0 (LocalVariables|GetTotalWeight)))
  (for _array_element_2 Spawn%20Data
    (bind _output_get (LocalVariables|SetRandomValue (- (LocalVariables|GetRandomValue) (.Spawnweight (Utilities|Struct|BreakFEnemySpawnData _array_element_2)))))
    (if (<= _output_get 0.0)
      (return (.NPCType (Utilities|Struct|BreakFEnemySpawnData _array_element_2)))))
  (Development|PrintString "weighted npc didnt work as intended, spawning default")
  (return "/Game/FGShooter/Npc/BP_Npc.BP_Npc_C"))