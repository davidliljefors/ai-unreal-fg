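; Torch actor that flickers its point light by animating the light's color.
; Construction script stores the light's starting color and sets a random timeline start time, likely to desynchronize torch instances.
; From BeginPlay, a timeline scales the red and green channels by a color multiplier curve, leaving blue unchanged.
; The timeline restarts on finish after a zero-length delay, looping the effect.
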(event EventBeginPlay
  (bind _basecolor (Variables|Default|GetBaseColor))
  (bind (_r _g _b) (Utilities|Struct|BreakLinearColor _basecolor))
  (bind _colormultiplier (Timeline|Timeline_0 Play)
    (:Update
      (Rendering|Components|Light|SetLightColor (Variables|Default|GetPointLight) (Math|Conversions|ToLinearColor(Vector) (Math|Vector|MakeVector (* (.X (Math|Vector|BreakVector _colormultiplier)) _r) (* (.Y (Math|Vector|BreakVector _colormultiplier)) _g) _b)) true))
    (:Finished
      (Utilities|FlowControl|Delay 0.0)
      (Timeline|Timeline_0 PlayFromStart))))

(event Collision|EventActorBeginOverlap
  (params (OtherActor :type Actor%20Object%20Reference)))

(fn ConstructionScript
  (Variables|Default|SetBaseColor (Rendering|Components|Light|GetLightColor (Variables|Default|GetPointLight)))
  (Components|Timeline|SetNewTime (Variables|Default|GetTimeline_0) (Math|Random|RandomFloatinRange 0.0 6.0)))