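; BP_Controller handles first-player input for the FGShooter game, driving movement, look, jump and crouch on the player character.
; Axis events move the character along its forward and right vectors and feed controller yaw and pitch.
; Jump and Crouch follow press and release, while ScrollJump fakes a short press by stopping the jump after a brief delay.
; Every event targets player character index 0 directly.
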(event Input|ActionEvents|InputActionJump
  (params (Key :type Key%20Structure))
  (bind _returnvalue (Game|GetPlayerCharacter 0))
  (:Pressed
    (Character|Jump _returnvalue))
  (:Released
    (Character|StopJumping _returnvalue)))

(event Input|ActionEvents|InputActionCrouch
  (params (Key :type Key%20Structure))
  (bind _returnvalue (Game|GetPlayerCharacter 0))
  (:Pressed
    (Character|Crouch _returnvalue))
  (:Released
    (Character|UnCrouch _returnvalue)))

(event Input|ActionEvents|InputActionScrollJump
  (params (Key :type Key%20Structure))
  (bind _returnvalue (Game|GetPlayerCharacter 0))
  (:Pressed
    (Character|Jump _returnvalue)
    (Utilities|FlowControl|Delay 0.05)
    (Character|StopJumping _returnvalue)))

(event Input|ActionEvents|InputActionFire
  (params (Key :type Key%20Structure)))

(event Input|AxisEvents|InputAxisMoveForward
  (params (AxisValue :type Float%20%28single-precision%29))
  (bind _returnvalue (Game|GetPlayerCharacter 0))
  (Pawn|Input|AddMovementInput _returnvalue (Transformation|GetActorForwardVector _returnvalue) AxisValue false))

(event Input|AxisEvents|InputAxisMoveRight
  (params (AxisValue :type Float%20%28single-precision%29))
  (bind _returnvalue (Game|GetPlayerCharacter 0))
  (Pawn|Input|AddMovementInput _returnvalue (Transformation|GetActorRightVector _returnvalue) AxisValue false))

(event Input|AxisEvents|InputAxisLookUp
  (params (AxisValue :type Float%20%28single-precision%29))
  (Pawn|Input|AddControllerPitchInput (Game|GetPlayerCharacter 0) AxisValue))

(event Input|AxisEvents|InputAxisTurn
  (params (AxisValue :type Float%20%28single-precision%29))
  (Pawn|Input|AddControllerYawInput (Game|GetPlayerCharacter 0) AxisValue))

(fn ConstructionScript)