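; BP_Door is a swinging door that opens away from an approaching BP_SourcePlayer and closes when no players remain in its trigger box.
; Box overlap events pick a target state, using a dot product to choose the swing direction.
; TransitionToState lerps the mesh between per-state rotations on a timeline, queuing requests that arrive mid-swing.
; The construction script applies the initial state's rotation, and a FirstPersonCharacter key check is left unconnected.
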(event OnComponentBeginOverlap(Box)
  (params (OverlappedComponent :type Primitive%20Component%20Object%20Reference) (OtherActor :type Actor%20Object%20Reference) (OtherComp :type Primitive%20Component%20Object%20Reference) (OtherBodyIndex :type Integer) (bFromSweep :type Boolean) (SweepResult :type Hit%20Result%20Structure%20%28by%20ref%29))
  ;[1 1 1] On Overlap, open the door in oppisite of direction of player
  (Utilities|IsPlayer OtherActor
    (:IsPlayer
      (Utilities|IsValid (Variables|Default|GetOverlappingPlayer)
        (:Is%20Not%20Valid
          (Variables|Default|SetOverlappingPlayer OtherActor)
          (CallFunction|TransitiontoState (select (> (Class|Actor|GetDotProductto OtherActor) 0.0) "NewEnumerator2" "NewEnumerator1")))))))

(event OnComponentEndOverlap(Box)
  (params (OverlappedComponent :type Primitive%20Component%20Object%20Reference) (OtherActor :type Actor%20Object%20Reference) (OtherComp :type Primitive%20Component%20Object%20Reference) (OtherBodyIndex :type Integer))
  ;[1 1 1] On end overlap, close the door
  (if (not (> (Utilities|Array|Length (Collision|GetOverlappingActors (Variables|Default|GetBox) "/Game/FGShooter/BP_SourcePlayer.BP_SourcePlayer_C" :!class /Script/Engine.PrimitiveComponent)) 0))
    (Utilities|IsPlayer OtherActor
      (:IsPlayer
        (Utilities|IsValid (Variables|Default|GetOverlappingPlayer)
          (:Is%20Valid
            (Variables|Default|SetOverlappingPlayer 0)
            (CallFunction|TransitiontoState "NewEnumerator0")))))))

(event Custom|TransitionToState
  (params (TargetState :type EDoorState%20Enum :default "NewEnumerator0"))
  ;[1 1 1] Animating the door to a target state
  (if (and (Utilities|Enum|NotEqual(Enum) TargetState (Variables|Default|GetState)) (not (Variables|Default|GetbTransitioning)))
    (Variables|Default|SetbStateQueued false)
    (Variables|Default|SetbTransitioning true)
    (Variables|Default|SetTargetState TargetState)
    (bind _alpha (Timeline|Timeline_0 PlayFromStart)
      (:Update
        (Transformation|SetRelativeRotation (Variables|Default|GetSM_Door) (Math|Rotator|Lerp(Rotator) (.Value (Utilities|Map|Find (Variables|Default|GetTargetRotationByState) (Variables|Default|GetState))) (.Value (Utilities|Map|Find (Variables|Default|GetTargetRotationByState) (Variables|Default|GetTargetState))) _alpha) false false))
      (:Finished
        (Variables|Default|SetState (Variables|Default|GetTargetState))
        (Variables|Default|SetbTransitioning false)
        (if (Variables|Default|GetbStateQueued)
          (CallFunction|TransitiontoState (Variables|Default|GetQueuedTargetState)))))
    (else
      (Variables|Default|SetQueuedTargetState TargetState)
      (Variables|Default|SetbStateQueued true))))

(fn ConstructionScript
  (Transformation|SetRelativeRotation (Variables|Default|GetSM_Door) (.Value (Utilities|Map|Find (Variables|Default|GetTargetRotationByState) (Variables|Default|GetState))) false false))