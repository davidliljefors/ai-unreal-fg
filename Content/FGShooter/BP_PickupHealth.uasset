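; BP_PickupHealth is a health pickup that heals the player and then removes itself from the level.
; Both overlap by an actor whose class is exactly BP_SourcePlayer and a Use event route into PickupHealth.
; That function casts to BP_SourcePlayer, plays a food crunch sound at the pickup, calls RecoverHealth with HealAmount and destroys the actor.
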(event Collision|EventActorBeginOverlap
  (params (OtherActor :type Actor%20Object%20Reference))
  (if (== (Utilities|GetClass OtherActor) "/Game/FGShooter/BP_SourcePlayer.BP_SourcePlayer_C")
    (CallFunction|PickupHealth OtherActor)))

(event EventUse
  (params (Sender :type Actor%20Object%20Reference))
  (CallFunction|PickupHealth Sender))

(fn ConstructionScript
  (|CallParentFunction))

(fn PickupHealth
  (params (Object :type Object%20Object%20Reference))
  (bind _asbp_source_player (Utilities|Casting|CastToBP_SourcePlayer Object))
  (Audio|PlaySoundatLocation "/Game/FGShooter/A_food_crunch.A_food_crunch" (Transformation|GetActorLocation) "0, 0, 0" 1.0 1.0 0.0 0 0 0)
  (Default|RecoverHealth _asbp_source_player (Variables|Default|GetHealAmount))
  (Actor|DestroyActor))