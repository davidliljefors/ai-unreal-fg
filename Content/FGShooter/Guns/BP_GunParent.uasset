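; Base first-person gun, used as a child actor of BP_SourcePlayer, handling hitscan fire, recoil and clip-based ammo.
; StartShooting and StopShooting toggle IsFiring; FireBullet, not called here, enforces fire rate and traces from the player camera.
; A hit with a bone name counts as an enemy, reporting AI damage and sending ShotMessage; other hits play surface effects.
; Reloading runs ReloadAmmo on an interruptible timer, starting automatically when shooting begins on an empty clip.
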(event Custom|Reload%20Gun
  ;[1 1 1] Reload gun, calls function ReloadAmmo after the time it takes to reload.
  (if (not (Variables|Default|GetbIsReloading))
    (Variables|Default|SetbIsReloading true)
    (if (> (Variables|Default|GetAmmoCurrent) 0)
      (if (< (Variables|Default|GetAmmoInClip) (Variables|Default|GetClipSize))
        (bind _returnvalue (Audio|SpawnSoundAttached (Variables|Default|GetReloadSound) (Variables|Default|GetDefaultSceneRoot) "None" "0, 0, 0" "0, 0, 0" "KeepRelativeOffset" false 1.0 1.0 0.0 0 0))
        (Variables|Default|SetCurrentReloadSound _returnvalue)
        (bind _returnvalue_2 (Utilities|Time|SetTimerbyFunctionName 0 (Utilities|String|MakeLiteralString "ReloadAmmo") (Variables|Default|GetReloadTime)))
        (Variables|Default|SetReloadHandle _returnvalue_2)
        (else
          (Variables|Default|SetbIsReloading false :!label _label)))
      (else
        (goto _label)))))

(event Custom|InterruptReload
  ;[1 1 1] Stops current reload from executing
  (Utilities|Time|ClearandInvalidateTimerbyHandle (Variables|Default|GetReloadHandle))
  (Variables|Default|SetbIsReloading false)
  (bind _currentreloadsound (Variables|Default|GetCurrentReloadSound)
    (:then
      (Audio|Components|Audio|Stop _currentreloadsound))
    (:else)))

(event Custom|FillAmmoPercent
  (params (Amount%20in%20percent :type Float%20%28single-precision%29))
  (Variables|Default|SetAmmoCurrent (Math|Integer|Min(Integer) (Math|Float|Round (+ (Math|Conversions|ToFloat(Integer) (Variables|Default|GetAmmoCurrent)) (* (Variables|Default|GetAmmoMax) Amount%20in%20percent))) (Variables|Default|GetAmmoMax))))

(event Custom|StopShooting
  (Variables|Default|SetbIsFiring false))

(event Custom|StartShooting
  (if (<= (Variables|Default|GetAmmoInClip) 0)
    (CallFunction|ReloadGun)
    (elif (not (Variables|Default|GetbIsReloading))
      (Variables|Default|SetbIsFiring true)
      (else
        (Variables|Default|SetbIsFiring false)))))

(fn ConstructionScript
  (Transformation|AttachComponentToComponent (Variables|Default|GetGun) (Variables|Default|GetArms) "GripPoint" "SnapToTarget" "KeepRelative" "KeepRelative" true)
  (Variables|Default|SetAmmoInClip (Variables|Default|GetClipSize)))

(fn FireBullet
  (bind _returnvalue (Actor|GetParentActor))
  (bind _bodyimpactsounds (Variables|Default|GetBodyImpactSounds))
  (bind _surfaceimpactsounds (Variables|Default|GetSurfaceImpactSounds))
  (bind _barrelend (Variables|Default|GetBarrelEnd))
  (bind _returnvalue_2 (Transformation|GetWorldTransform _barrelend))
  (if (not (Variables|Default|GetbIsReloading))
    (if (> (Variables|Default|GetAmmoInClip) 0)
      (bind _asbp_source_player (Utilities|Casting|CastToBP_SourcePlayer (Actor|GetParentActor))
        (:then
          (if (>= (Utilities|Time|GetTimeSeconds) (+ (* (Variables|Default|GetFireRate) 0.9) (Variables|Default|GetLastShotTimestamp)))
            (Variables|Default|SetLastShotTimestamp (Utilities|Time|GetTimeSeconds))
            (Math|Integer|DecrementInt (Variables|Default|GetAmmoInClip)
              (:%20%20
                (Animation|Montage|MontagePlay (Components|SkeletalMesh|GetAnimInstance (Variables|Default|GetArms)) "/Game/FirstPerson/Animations/FirstPersonFire_Montage_2.FirstPersonFire_Montage_2" 1.0 "MontageLength" 0.0 true)
                (Audio|PlaySoundatLocation (Variables|Default|GetFireSound) (.location _returnvalue_2) "0, 0, 0" 0.7 1.0 0.0 0 "/Game/MilitaryWeapSilver/Sound/Rifle/Wavs/concurrency.concurrency" 0)
                (Class|AISenseHearing|ReportNoiseEvent (.location _returnvalue_2) 1.0 _asbp_source_player 0.0 "None")
                (Effects|SpawnEmitteratLocation "/Game/MilitaryWeapSilver/FX/P_AssaultRifle_MuzzleFlash.P_AssaultRifle_MuzzleFlash" (.location _returnvalue_2) (.rotation _returnvalue_2) "0.500000,0.500000,0.500000")
                (bind (_outhit _returnvalue_3) (Collision|LineTraceByChannel (Transformation|GetWorldLocation (Variables|/Game/FGShooter/BP_SourcePlayer.BP_SourcePlayer_C|GetCamera _asbp_source_player)) (+ (Transformation|GetWorldLocation (Variables|/Game/FGShooter/BP_SourcePlayer.BP_SourcePlayer_C|GetCamera _asbp_source_player)) (* (Math|Vector|GetForwardVector (Variables|/Game/FGShooter/BP_SourcePlayer.BP_SourcePlayer_C|GetCamera _asbp_source_player)) (LocalVariables|GetLine%20Trace%20Range))) "TraceTypeQuery2" false (Utilities|Array|MakeArray (Actor|GetParentActor)) "None"))
                (CallFunction|AddRecoil)
                (if _returnvalue_3
                  (if (Utilities|Name|NotEqual(Name) (.hitbonename _outhit) "None")
                    (Class|AISenseDamage|ReportDamageEvent (.hitactor _outhit) _returnvalue (Variables|Default|GetGunDamage) (.tracestart _outhit))
                    (Class|BPIInteractable|Shot(Message) (.hitactor _outhit) (Variables|Default|GetGunDamage) _returnvalue (.impactpoint _outhit) (.hitbonename _outhit))
                    (Audio|PlaySoundatLocation (Utilities|Array|Get(acopy) _bodyimpactsounds (Math|Random|RandomIntegerinRange 0 (- (Utilities|Array|Length _bodyimpactsounds) 1))) (.impactpoint _outhit) "0, 0, 0" 1.0 1.0 0.0 "/Game/MilitaryWeapSilver/Sound/SniperRifle/Wavs/AttenuationTest.AttenuationTest" 0 0)
                    (return)
                    (else
                      (Audio|PlaySoundatLocation (Utilities|Array|Get(acopy) _surfaceimpactsounds (Math|Random|RandomIntegerinRange 0 (- (Utilities|Array|Length _surfaceimpactsounds) 1))) (.impactpoint _outhit) "0, 0, 0" 1.0 1.0 0.0 "/Game/MilitaryWeapSilver/Sound/SniperRifle/Wavs/AttenuationTest.AttenuationTest" 0 0)
                      (Effects|SpawnEmitteratLocation "/Game/MilitaryWeapSilver/FX/P_Impact_Metal_Small_01.P_Impact_Metal_Small_01" (.impactpoint _outhit) (Math|Conversions|RotationFromXVector (Math|Vector|RotateVector (.normal _outhit) (Math|Conversions|RotationFromXVector "0.000000,90.000000, 0"))))
                      (return)))
                  (else
                    (return)))))
            (else
              (return))))
        (:CastFailed
          (return)))
      (else
        (return)))
    (else
      (return))))

(fn Reload
  (if (> (Variables|Default|GetAmmoCurrent) 0)
    (if (< (Variables|Default|GetAmmoInClip) (Variables|Default|GetClipSize))
      (if (>= (Variables|Default|GetAmmoCurrent) (- (Variables|Default|GetClipSize) (Variables|Default|GetAmmoInClip)))
        (Variables|Default|SetAmmoCurrent (+ (Variables|Default|GetAmmoCurrent) (Variables|Default|GetAmmoInClip)))
        (Variables|Default|SetAmmoInClip (Variables|Default|GetClipSize))
        (Variables|Default|SetAmmoCurrent (- (Variables|Default|GetAmmoCurrent) (Variables|Default|GetClipSize)))
        (else
          (Variables|Default|SetAmmoInClip (+ (Variables|Default|GetAmmoInClip) (Variables|Default|GetAmmoCurrent)))
          (Variables|Default|SetAmmoCurrent 0)))
      (else
        (return)))
    (else
      (return))))

(fn AddRecoil
  (bind _returnvalue (Game|GetPlayerCharacter 0))
  (Pawn|Input|AddControllerPitchInput _returnvalue (Math|Random|RandomFloatinRange -0.2 -0.25))
  (Pawn|Input|AddControllerYawInput _returnvalue (Math|Random|RandomFloatinRange -0.15 0.15))
  (return))

(fn ReloadAmmo
  (if (>= (Variables|Default|GetAmmoCurrent) (- (Variables|Default|GetClipSize) (Variables|Default|GetAmmoInClip)))
    (Variables|Default|SetAmmoCurrent (+ (Variables|Default|GetAmmoCurrent) (Variables|Default|GetAmmoInClip)))
    (Variables|Default|SetAmmoInClip (Variables|Default|GetClipSize))
    (Variables|Default|SetAmmoCurrent (- (Variables|Default|GetAmmoCurrent) (Variables|Default|GetClipSize)))
    (Variables|Default|SetbIsReloading false)
    (return)
    (else
      (Variables|Default|SetAmmoInClip (+ (Variables|Default|GetAmmoInClip) (Variables|Default|GetAmmoCurrent)))
      (Variables|Default|SetAmmoCurrent 0)
      (Variables|Default|SetbIsReloading false)
      (return))))