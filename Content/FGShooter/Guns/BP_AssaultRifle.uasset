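; BP_AssaultRifle is an automatic gun that keeps firing from StartShooting until StopShooting.
; StartShooting calls the parent, fires one bullet immediately, then starts a looping timer on Fire Bullet that uses FireRate as the interval in seconds.
; StopShooting calls the parent and clears the stored GunTimer handle to end the burst.
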(event EventStartShooting
  (|CallParentFunction)
  (CallFunction|FireBullet)
  (bind _returnvalue (Utilities|Time|SetTimerbyFunctionName 0 "Fire Bullet" (Variables|Default|GetFireRate) true))
  (Variables|Default|SetGun%20Timer _returnvalue))

(event EventStopShooting
  (|CallParentFunction)
  (Utilities|Time|ClearandInvalidateTimerbyHandle (Variables|Default|GetGun%20Timer)))

(fn ConstructionScript
  (|CallParentFunction))