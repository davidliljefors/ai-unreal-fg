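; BP_Sniper is a sniper rifle gun Blueprint that extends a parent gun class's shooting behavior.
; StartShooting runs the parent logic and calls FireBullet, then, if not reloading, plays two timed bolt-cycle style reload sounds using delays.
; Both sounds play at the world origin rather than at the weapon.
; StopShooting and the construction script only defer to the parent.
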(event EventStartShooting
  (|CallParentFunction)
  (CallFunction|FireBullet)
  (if (not (Variables|Default|GetbIsReloading))
    (Utilities|FlowControl|Delay 0.5)
    (Audio|PlaySoundatLocation "/Game/MilitaryWeapSilver/Sound/SniperRifle/Wavs/SniperRifle_Reload01.SniperRifle_Reload01" "0, 0, 0" "0, 0, 0" 1.0 1.0 0.0 0 0 0)
    (Utilities|FlowControl|Delay 1.0)
    (Audio|PlaySoundatLocation "/Game/MilitaryWeapSilver/Sound/SniperRifle/Wavs/SniperRifle_ReloadInsert03.SniperRifle_ReloadInsert03" "0, 0, 0" "0, 0, 0" 1.0 1.0 0.0 0 0 0)))

(event EventStopShooting
  (|CallParentFunction))

(fn ConstructionScript
  (|CallParentFunction))