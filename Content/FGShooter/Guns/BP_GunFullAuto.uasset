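; BP_GunFullAuto is a full-automatic gun Blueprint that keeps firing bullets while shooting is active.
; On StartShooting it calls the parent logic, fires one bullet immediately, then starts a looping timer that calls Fire Bullet at the FireRate interval.
; StopShooting calls the parent logic and clears that timer to end the automatic fire.
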(event EventStartShooting
  (|CallParentFunction)
  (CallFunction|FireBullet)
  (bind _returnvalue (Utilities|Time|SetTimerbyFunctionName 0 "Fire Bullet" (Variables|Default|GetFireRate) true))
  (Variables|Default|SetGunTimer _returnvalue))

(event EventStopShooting
  (|CallParentFunction)
  (Utilities|Time|ClearandInvalidateTimerbyHandle (Variables|Default|GetGunTimer)))

(fn ConstructionScript
  (|CallParentFunction))