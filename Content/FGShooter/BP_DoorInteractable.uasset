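; Interactable swinging door that toggles on Use, picking one of two open directions from which side of the door the sender is on.
; A timeline lerps the mesh rotation between per-state rotations from a map, which the construction script also applies to show the starting state.
; Use during a swing toggles from the target state and queues the result to play when the current transition finishes.
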(event Custom|TransitionToState
  (params (TargetState :type EDoorState%20Enum :default "NewEnumerator0"))
  ;[1 1 1] Animating the door to a target state
  (if (and (Utilities|Enum|NotEqual(Enum) TargetState (Variables|Default|GetState)) (not (Variables|Default|GetbTransitioning)))
    (Variables|Default|SetbStateQueued false)
    (Variables|Default|SetbTransitioning true)
    (Variables|Default|SetTargetState TargetState)
    (bind _alpha (Timeline|Timeline_0 PlayFromStart)
      (:Update
        (Transformation|SetRelativeRotation (Variables|Default|GetSM_Door) (Math|Rotator|Lerp(Rotator) (.Value (Utilities|Map|Find (Variables|Default|GetTargetRotationByState) (Variables|Default|GetState))) (.Value (Utilities|Map|Find (Variables|Default|GetTargetRotationByState) (Variables|Default|GetTargetState))) _alpha) false false))
      (:Finished
        (Variables|Default|SetState (Variables|Default|GetTargetState))
        (Variables|Default|SetbTransitioning false)
        (if (Variables|Default|GetbStateQueued)
          (CallFunction|TransitiontoState (Variables|Default|GetQueuedTargetState)))))
    (else
      (Variables|Default|SetQueuedTargetState TargetState)
      (Variables|Default|SetbStateQueued true))))

(event EventUse
  (params (Sender :type Actor%20Object%20Reference))
  (if (Variables|Default|GetbTransitioning)
    (if (Utilities|Enum|Equal(Enum) (Variables|Default|GetTargetState) "NewEnumerator0")
      (CallFunction|TransitiontoState (select (> (Class|Actor|GetDotProductto Sender) 0.0) "NewEnumerator2" "NewEnumerator1") :!label _label)
      (else
        (CallFunction|TransitiontoState "NewEnumerator0" :!label _label_2)))
    (elif (Utilities|Enum|Equal(Enum) (Variables|Default|GetState) "NewEnumerator0")
      (goto _label)
      (else
        (goto _label_2)))))

(fn ConstructionScript
  (Transformation|SetRelativeRotation (Variables|Default|GetSM_Door) (.Value (Utilities|Map|Find (Variables|Default|GetTargetRotationByState) (Variables|Default|GetState))) false false))