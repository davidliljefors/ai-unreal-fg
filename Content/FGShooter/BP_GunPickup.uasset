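; Gun pickup that gives BP_SourcePlayer a secondary weapon, triggered by actor overlap or a Use event.
; The construction script displays the configured GunMesh on the skeletal mesh.
; Both triggers call PickupGun, which only acts when the player's SecondaryWeapon child actor slot is empty.
; It then sets that slot's class to Gun, plays a raise sound at the player and destroys the pickup.
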(event EventUse
  (params (Sender :type Actor%20Object%20Reference))
  (CallFunction|PickupGun Sender))

(event Collision|EventActorBeginOverlap
  (params (OtherActor :type Actor%20Object%20Reference))
  (CallFunction|PickupGun OtherActor))

(fn ConstructionScript
  (|CallParentFunction)
  (Class|SkinnedMeshComponent|SetSkeletalMesh (Variables|Default|GetSkeletalMesh) (Variables|Default|GetGun%20Mesh) true))

(fn PickupGun
  (params (Object :type Object%20Object%20Reference))
  (bind _asbp_source_player (Utilities|Casting|CastToBP_SourcePlayer Object))
  (Variables|/Script/Engine.ChildActorComponent|GetChildActor (Variables|/Game/FGShooter/BP_SourcePlayer.BP_SourcePlayer_C|GetSecondaryWeapon _asbp_source_player)
    (:then)
    (:else
      (ChildActorComponent|SetChildActorClass (Variables|/Game/FGShooter/BP_SourcePlayer.BP_SourcePlayer_C|GetSecondaryWeapon _asbp_source_player) (Variables|Default|GetGun))
      (Audio|PlaySoundatLocation "/Game/MilitaryWeapSilver/Sound/SniperRifle/Wavs/SniperRifle_Raise.SniperRifle_Raise" (Transformation|GetActorLocation _asbp_source_player) "0, 0, 0" 1.0 1.0 0.0 0 0 0)
      (Actor|DestroyActor))))