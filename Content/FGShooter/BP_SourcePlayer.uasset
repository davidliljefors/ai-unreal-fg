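; Player character for a shooter, handling health, interaction and two child-actor weapons attached to the camera.
; Fire, reload and switch inputs drive the active BP_GunParent, with switching toggling visibility and interrupting reloads.
; Use line-traces from the camera and sends UseMessage to the hit actor; the hover trace is disconnected.
; Lethal shots call LoseGame on BP_GameState, hide weapons and switch to RagdollCam; ragdoll physics is disconnected.
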(event Custom|Recover%20Health
  (params (Amount :type Float%20%28single-precision%29))
  (Variables|Default|SetHealth (Math|Float|Min(Float) (+ Amount (Variables|Default|GetHealth)) (Variables|Default|GetMaxHealth))))

(event EventShot
  (params (Damage :type Float%20%28single-precision%29) (Instigator :type Actor%20Object%20Reference) (Hit%20Point :type Vector :default "0, 0, 0") (Bone%20Hit :type Name :default "None"))
  ;[1 1 1] Get shot
  (Variables|Default|SetHealth (- (Variables|Default|GetHealth) Damage))
  (Audio|PlaySoundatLocation "/Game/FGShooter/A_player_hit.A_player_hit" (Transformation|GetActorLocation) "0, 0, 0" 1.0 1.0 0.0 0 0 0)
  (if (<= (Variables|Default|GetHealth) 0.0)
    (bind _asbp_game_state (Utilities|Casting|CastToBP_GameState (Game|GetGameState)))
    (Default|LoseGame _asbp_game_state)
    (Variables|Default|SetbIsDead true)
    (Utilities|DieasRagdoll Hit%20Point 2e+06)))

(event EventBeginPlay
  ;[1 1 1] Default to primary weapon
  (Variables|Default|SetActiveWeapon (Variables|Default|GetPrimaryWeapon)))

(event EventTick
  (params (DeltaSeconds :type Float%20%28single-precision%29))
  ;[1 1 1] interaction tick
)

(event Input|ActionEvents|InputActionFire
  (params (Key :type Key%20Structure))
  ;[1 1 1] Fire Weapon
  (:Pressed
    (if (not (Variables|Default|GetbIsDead))
      (bind _asbp_gun_parent (Utilities|Casting|CastToBP_GunParent (Variables|/Script/Engine.ChildActorComponent|GetChildActor (Variables|Default|GetActiveWeapon))))
      (Default|StartShooting _asbp_gun_parent)))
  (:Released
    (Default|StopShooting _asbp_gun_parent)))

(event Input|ActionEvents|InputActionUse
  (params (Key :type Key%20Structure))
  (bind _interactiondistance (Variables|Default|GetInteractionDistance))
  (bind (_origin _forward) (Utilities|CameraOrigin+Forward _interactiondistance))
  ;[1 1 1] Interact with interactables
  (:Pressed
    (if (not (Variables|Default|GetbIsDead))
      (bind (_outhit _returnvalue) (Collision|LineTraceByChannel _origin _forward "TraceTypeQuery2" false 0 "ForDuration" true "(R=0.000000,G=0.973963,B=1.000000,A=1.000000)" "(R=1.000000,G=0.881067,B=0.000000,A=1.000000)" 2.0))
      (if _returnvalue
        (Class|BPIInteractable|Use(Message) (.HitActor (Collision|BreakHitResult _outhit)) self)))))

(event Input|ActionEvents|InputActionReload
  (params (Key :type Key%20Structure))
  ;[1 1 1] Reload weapon
  (:Pressed
    (if (not (Variables|Default|GetbIsDead))
      (bind _asbp_gun_parent (Utilities|Casting|CastToBP_GunParent (Variables|/Script/Engine.ChildActorComponent|GetChildActor (Variables|Default|GetActiveWeapon))))
      (Default|ReloadGun _asbp_gun_parent))))

(event Input|ActionEvents|InputActionWeaponSwitch
  (params (Key :type Key%20Structure))
  (bind _returnvalue (Transformation|GetActorLocation))
  ;[1 1 1] Switch weapons, cancels reload if needed.
  (:Pressed
    (if (not (Variables|Default|GetbIsDead))
      (Variables|/Script/Engine.ChildActorComponent|GetChildActor (Variables|Default|GetSecondaryWeapon)
        (:then
          (bind _asbp_gun_parent (Utilities|Casting|CastToBP_GunParent (Variables|/Script/Engine.ChildActorComponent|GetChildActor (Variables|Default|GetActiveWeapon))))
          (if (Variables|/Game/FGShooter/Guns/BP_GunParent.BP_GunParent_C|GetbIsReloading _asbp_gun_parent)
            (Default|InterruptReload _asbp_gun_parent))
          (Default|StopShooting _asbp_gun_parent)
          (bind _isa (Utilities|FlowControl|FlipFlop)
            (:A
              (Variables|Default|SetActiveWeapon (Variables|Default|GetSecondaryWeapon))
              (Audio|PlaySoundatLocation "/Game/MilitaryWeapSilver/Sound/Rifle/Wavs/Rifle_Raise.Rifle_Raise" _returnvalue "0, 0, 0" 1.0 1.0 0.0 0 0 0))
            (:B
              (Variables|Default|SetActiveWeapon (Variables|Default|GetPrimaryWeapon))
              (Audio|PlaySoundatLocation "/Game/MilitaryWeapSilver/Sound/Rifle/Wavs/Rifle_Lower.Rifle_Lower" _returnvalue "0, 0, 0" 1.0 1.0 0.0 0 0 0)))
          (Development|SetHiddeninGame (Variables|Default|GetPrimaryWeapon) _isa true)
          (Development|SetHiddeninGame (Variables|Default|GetSecondaryWeapon) (not _isa) true))
        (:else)))))

(fn ConstructionScript
  (Transformation|AttachComponentToComponent (Variables|Default|GetPrimaryWeapon) (Variables|Default|GetCamera) "None" "KeepWorld" "KeepWorld" "KeepWorld" true)
  (Collision|SetCollisionEnabled (Variables|Character|GetMesh) "NoCollision")
  (Transformation|AttachComponentToComponent (Variables|Default|GetSecondaryWeapon) (Variables|Default|GetCamera) "None" "KeepWorld" "KeepWorld" "KeepWorld" true))