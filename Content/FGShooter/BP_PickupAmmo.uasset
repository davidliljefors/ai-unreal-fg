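; Ammo pickup actor that refills a player's weapons when a BP_SourcePlayer overlaps it or triggers its Use event.
; Both events call PickupAmmo, which plays a pickup sound, then calls FillAmmoPercent on the BP_GunParent child actors of the primary and secondary weapons.
; The pickup destroys itself afterward, though a failed primary gun cast exits early and leaves it in the world.
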(event EventUse
  (params (Sender :type Actor%20Object%20Reference))
  (if (== (Utilities|GetClass Sender) "/Game/FGShooter/BP_SourcePlayer.BP_SourcePlayer_C")
    (Utilities|PickupAmmo Sender)))

(event Collision|EventActorBeginOverlap
  (params (OtherActor :type Actor%20Object%20Reference))
  (if (== (Utilities|GetClass OtherActor) "/Game/FGShooter/BP_SourcePlayer.BP_SourcePlayer_C")
    (Utilities|PickupAmmo OtherActor)))

(fn ConstructionScript
  (|CallParentFunction))