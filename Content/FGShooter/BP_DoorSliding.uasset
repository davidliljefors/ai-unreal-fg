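; BP_DoorSliding is a sliding door that toggles between closed and lowered, open states.
; The construction script caches the Cube's world location as the start position.
; ToggleDoor flips IsOpen and plays or reverses a timeline, whose alpha lerps the Cube between that position and a fixed downward Z offset, without sweeping.
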(event Custom|ToggleDoor
  (bind _startposition (Variables|Default|GetStartPosition))
  (if (Variables|Default|GetbIsOpen)
    (Variables|Default|SetbIsOpen false)
    (bind _alpha (Timeline|Timeline_0 Reverse)
      (:Update
        (Transformation|SetWorldLocation (Variables|Default|GetCube) (Math|Vector|Lerp(Vector) _startposition (+ _startposition (Math|Vector|MakeVector 0.0 0.0 -299.0)) _alpha) false false)))
    (else
      (Variables|Default|SetbIsOpen true)
      (Timeline|Timeline_0 Play))))

(fn ConstructionScript
  (Variables|Default|SetStartPosition (Transformation|GetWorldLocation (Variables|Default|GetCube))))